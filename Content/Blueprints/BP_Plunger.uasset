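; Pinball-style plunger that pulls back while Space is held and returns when released, launching the ball it hits.
; Each Tick reads the IsSpacePressed flag and interpolates the Plunger's world location toward EndPosition or InitialPosition, without sweeping.
; On Hit, a BP_Ball receives an impulse along the hit normal scaled by ImpulseForce, independent of pull distance.
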(event `self.ReceiveTick`
  (params (DeltaSeconds :type "Float (single-precision)"))
  ;[1 1 1] Alt click deletes connection
  (if (`self.IsSpacePressed`)
    (`self.PlungerPull` DeltaSeconds (`self.Speed`))
    (else
      (`self.PlungerThrust` DeltaSeconds (`self.Speed`)))))

(event `self.ReceiveHit`
  (params (MyComp :type "PrimitiveComponent Object Reference") (Other :type "Actor Object Reference") (OtherComp :type "PrimitiveComponent Object Reference") (bSelfMoved :type Boolean) (HitLocation :type "Vector Structure") (HitNormal :type "Vector Structure") (NormalImpulse :type "Vector Structure") (Hit :type "HitResult Structure (by ref)"))
  (bind _asbp_ball (cast `/Game/Blueprints/BP_Ball` Other))
  (`PrimitiveComponent.AddImpulse` (`/Game/Blueprints/BP_Ball.Ball` _asbp_ball) (* (`self.Impulse Force`) HitNormal) "None" false))

(fn `PlungerPull`
  (params (Delta :type "Float (double-precision)") (Speed :type "Float (double-precision)"))
  (`SceneComponent.K2_SetWorldLocation` (`self.Plunger`) (`KismetMathLibrary.VInterpTo` (`SceneComponent.K2_GetComponentLocation` (`self.Plunger`)) (`SceneComponent.K2_GetComponentLocation` (`self.End Position`)) Delta Speed) false false))

(fn `PlungerThrust`
  (params (Delta :type "Float (double-precision)") (Speed :type "Float (double-precision)"))
  (`SceneComponent.K2_SetWorldLocation` (`self.Plunger`) (`KismetMathLibrary.VInterpTo` (`SceneComponent.K2_GetComponentLocation` (`self.Plunger`)) (`SceneComponent.K2_GetComponentLocation` (`self.Initial position`)) Delta Speed) false false))

(fn `UserConstructionScript`)